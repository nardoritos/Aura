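; BP_Aura_MainMenu is the main menu scene actor, animating a floating fireball effect and title widget.
; On BeginPlay it caches both components' start locations, plays menu music, shows WBP_MainMenu and switches to UI-only input with a visible cursor.
; Each Tick advances a timer that wraps at 2π and drives a sine-wave vertical bob on both components, each with its own amplitude.
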(event EventBeginPlay
  (bind _returnvalue (Game|GetPlayerController 0))
  (Variables|Default|SetFireballInitialLocation (Transformation|GetWorldLocation (Variables|Default|GetFireBallSystem)))
  (Variables|Default|SetWidgetInitialLocation (Transformation|GetWorldLocation (Variables|Default|GetTitleWidget)))
  (bind _returnvalue_2 (Audio|SpawnSound2D "/Game/Assets/Sounds/Music/Music_MainMenu.Music_MainMenu" 1.0 1.0 0.0 0))
  (Variables|Default|SetMainMenuMusic _returnvalue_2)
  (bind _returnvalue_3 (UserInterface|CreateWidget "/Game/Blueprints/UI/MainMenu/WBP_MainMenu.WBP_MainMenu_C"))
  (UserInterface|Viewport|AddtoViewport _returnvalue_3 0)
  (Input|SetInputModeUIOnly _returnvalue _returnvalue_3 "DoNotLock" false)
  (Variables|/Script/Engine.PlayerController|SetbShowMouseCursor _returnvalue true))

(event Collision|EventActorBeginOverlap
  (params (OtherActor :type Actor%20Object%20Reference)))

(event EventTick
  (params (DeltaSeconds :type Float%20%28single-precision%29))
  (CallFunction|UpdateTime DeltaSeconds)
  (CallFunction|MoveFireBall)
  (CallFunction|MoveTitleWidget))

(fn ConstructionScript)

(fn UpdateTime
  (params (DeltaSeconds :type Float%20%28double-precision%29))
  (bind _output_get (Variables|Default|SetTime (+ DeltaSeconds (Variables|Default|GetTime))))
  (if (> _output_get (* (Math|Trig|GetPI) 2.0))
    (Variables|Default|SetTime 0.0)))

(fn MoveFireBall
  (bind _fireballinitiallocation (Variables|Default|GetFireballInitialLocation))
  (Transformation|SetWorldLocation (Variables|Default|GetFireBallSystem) (Math|Vector|MakeVector (.x _fireballinitiallocation) (.y _fireballinitiallocation) (+ (.z _fireballinitiallocation) (* (Math|Trig|Sin(Radians) (Variables|Default|GetTime)) (Variables|Default|GetFireballAmplitude)))) false false))

(fn MoveTitleWidget
  (bind _widgetinitiallocation (Variables|Default|GetWidgetInitialLocation))
  (Transformation|SetWorldLocation (Variables|Default|GetTitleWidget) (Math|Vector|MakeVector (.x _widgetinitiallocation) (.y _widgetinitiallocation) (+ (.z _widgetinitiallocation) (* (Math|Trig|Sin(Radians) (Variables|Default|GetTime)) (Variables|Default|GetWidgetAmplitude)))) false false))