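; BP_SlingshotRock is the rock projectile for an enemy slingshot ability, tumbling visually while in play.
; BeginPlay rolls a random spin rate for each axis, which Tick scales by delta time to rotate RockMesh locally.
; After a brief delay from BeginPlay, the Sphere component's collision switches to query-only.
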(event EventBeginPlay
  (bind _returnvalue (Math|Random|RandomFloatinRange -5e+02 5e+02))
  (Variables|Default|SetYawRotationRate _returnvalue)
  (Variables|Default|SetPitchRotationRate _returnvalue)
  (Variables|Default|SetRollRotationRate _returnvalue)
  (Utilities|FlowControl|Delay 0.15)
  (Collision|SetCollisionEnabled (Variables|Default|GetSphere) "QueryOnly"))

(event EventTick
  (params (DeltaSeconds :type Float%20%28single-precision%29))
  (bind _yawrotationrate (Variables|Default|GetYawRotationRate))
  (bind _pitchrotationrate (Variables|Default|GetPitchRotationRate))
  (bind _rollrotationrate (Variables|Default|GetRollRotationRate))
  (bind _returnvalue (Math|Vector|MakeVector _yawrotationrate _pitchrotationrate _rollrotationrate))
  (bind _returnvalue_2 (* DeltaSeconds _returnvalue))
  (Transformation|AddLocalRotation (Variables|Default|GetRockMesh) (Math|Rotator|MakeRotator (.x _returnvalue_2) (.y _returnvalue_2) (.z _returnvalue_2)) false false))

(fn ConstructionScript)