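; Enemy melee attack Gameplay Ability that faces the combat target and plays a random tagged attack montage from the avatar.
; On the montage's gameplay event, it finds live players within a small radius of the tagged combat socket.
; Non-friends take damage and show blood; any hit fires one MeleeImpact cue carrying the montage tag.
; The ability ends after that hit check, or when the montage completes, is interrupted or is cancelled.
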(event Ability|EventActivateAbility
  (bind _returnvalue (Ability|GetAvatarActorfromActorInfo))
  (bind _returnvalue_2 (Ability|GetAvatarActorfromActorInfo))
  (bind _returnvalue_3 (Ability|GetAvatarActorfromActorInfo))
  (Variables|Default|SetTargetActor 0)
  (Variables|Default|SetHasHitTarget false)
  (bind _returnvalue_4 (Class|EnemyInterface|GetCombatTarget(Message) _returnvalue))
  (Class|CombatInterface|UpdateFacingTarget(Message) _returnvalue (Transformation|GetActorLocation _returnvalue_4))
  (bind _returnvalue_5 (Class|CombatInterface|GetAttackMontages(Message) (Ability|GetAvatarActorfromActorInfo)))
  (Variables|Default|SetTaggedMontage (Class|AuraDamageGameplayAbility|GetRandomTaggedMontagefromArray _returnvalue_5))
  (|PlayMontageandWaitProxy "None" (.Montage (Utilities|Struct|BreakTaggedMontage (Variables|Default|GetTaggedMontage))) 1.0 "None" true 1.0 0.0 false
    (:then
      (Ability|Tasks|WaitGameplayEvent (.MontageTag (Utilities|Struct|BreakTaggedMontage (Variables|Default|GetTaggedMontage))) 0
        (:EventReceived
          (bind _returnvalue_6 (Class|CombatInterface|GetCombatSocketLocation(Message) _returnvalue_3 (.SocketTag (Utilities|Struct|BreakTaggedMontage (Variables|Default|GetTaggedMontage)))))
          (bind _output_get (Variables|Default|SetCombatSocketLocation _returnvalue_6))
          (bind _outoverlappingactors (Class|AuraAbilitySystemLibrary|GetLivePlayersWithinRadius _returnvalue_3 (Utilities|Array|MakeArray _returnvalue_3) 45.0 _output_get))
          (for _array_element _outoverlappingactors
            (Variables|Default|SetTargetActor _array_element)
            (if (Class|AuraAbilitySystemLibrary|IsNotFriend (Ability|GetAvatarActorfromActorInfo) (Variables|Default|GetTargetActor))
              (Class|AuraAbilitySystemLibrary|ApplyDamageEffect (Class|AuraDamageGameplayAbility|MakeDamageEffectParamsfromClassDefaults (Variables|Default|GetTargetActor) "0, 0, 0" false "0, 0, 0" false "0, 0, 0" false 0.0))
              (Variables|Default|SetHasHitTarget true)
              (Class|CombatInterface|GetBloodEffect(Message) (Variables|Default|GetTargetActor))))
          (Utilities|FlowControl|Sequence
            (:then_0
              (if (Variables|Default|GetHasHitTarget)
                (bind _returnvalue_7 (Class|EnemyInterface|GetCombatTarget(Message) _returnvalue_2))
                (Class|GameplayAbility|ExecuteGameplayCuewithParams "(TagName=\"GameplayCue.MeleeImpact\")" (Ability|GameplayCue|MakeGameplayCueParameters :AggregatedSourceTags (GameplayTags|MakeGameplayTagContainerfromTag (Utilities|Struct|BreakTaggedMontage (Variables|Default|GetTaggedMontage))) :Location (Variables|Default|GetCombatSocketLocation) :EffectCauser _returnvalue_2 :SourceObject _returnvalue_7))))
            (:then_1
              (Ability|EndAbility))))))
    (:OnCompleted
      (Ability|EndAbility :!label _label))
    (:OnInterrupted
      (goto _label))
    (:OnCancelled
      (goto _label))))