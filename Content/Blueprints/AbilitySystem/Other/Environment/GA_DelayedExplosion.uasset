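; GA_DelayedExplosion is a gameplay ability that triggers a telegraphed radial explosion on the ground at the avatar's location.
; A vertical trace finds the impact point, where a radial indicator sized to the damage radius shows for the activation delay.
; After the delay, live players in range, excluding the avatar, receive radial damage effects with a pitch override, and a radius-scaled fire explosion Niagara effect spawns.
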(event Ability|EventActivateAbility
  (bind _returnvalue (Ability|GetAvatarActorfromActorInfo))
  (bind _returnvalue_2 (Ability|GetAvatarActorfromActorInfo))
  (bind _returnvalue_3 (Transformation|GetActorLocation _returnvalue_2))
  (Ability|CommitAbility)
  (bind _outhit (Collision|LineTraceByChannel (+ _returnvalue_3 "0.000000,0.000000,250.000000") (- _returnvalue_3 "0.000000,0.000000,250.000000") "TraceTypeQuery1" false 0 "None"))
  (if (.bBlockingHit (Collision|BreakHitResult _outhit))
    (bind _output_get (Variables|Default|SetImpactLocation (.ImpactPoint (Collision|BreakHitResult _outhit))))
    (bind _returnvalue_4 (Game|SpawnActorfromClass "/Game/Blueprints/AbilitySystem/Other/Environment/BP_RadialIndicator.BP_RadialIndicator_C" (Math|Transform|MakeTransform _output_get "0, 0, 0" "1.000000,1.000000,1.000000") "AlwaysSpawn" "MultiplyWithRoot" 0 (Variables|Default|GetRadialDamageOuterRadius) 0))
    (bind _output_get_2 (Variables|Default|SetRadialIndicator _returnvalue_4))
    (Actor|SetLifeSpan _output_get_2 (Variables|Default|GetActivationDelay))
    (Utilities|FlowControl|Delay (Variables|Default|GetActivationDelay))
    (bind _outoverlappingactors (Class|AuraAbilitySystemLibrary|GetLivePlayersWithinRadius _returnvalue (Utilities|Array|MakeArray _returnvalue) (Variables|Default|GetRadialDamageOuterRadius) (Variables|Default|GetImpactLocation) false))
    (for _array_element _outoverlappingactors
      (Class|AuraAbilitySystemLibrary|ApplyDamageEffect (Class|AuraDamageGameplayAbility|MakeDamageEffectParamsfromClassDefaults _array_element (Variables|Default|GetImpactLocation) false "0, 0, 0" false "0, 0, 0" true 2e+01)))
    (Niagara|SpawnSystematLocation "/Game/Assets/Effects/Projectiles/FireExplosion/NS_FireExplosion1_Local.NS_FireExplosion1_Local" (Variables|Default|GetImpactLocation) "0, 0, 0" (Math|Conversions|ToVector(Float) (/ (Variables|Default|GetRadialDamageOuterRadius) 5e+01)))
    (Ability|EndAbility)
    (else
      (Ability|EndAbility))))