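; Passive gameplay ability that turns Attributes gameplay events into Gameplay Effects applied to its owner.
; On activation it waits for events under the Attributes tag, including child tags, and builds a spec from EventBasedEffectClass for each one received.
; It sets the SetByCaller magnitude of the exactly matching entry in EventTags to the payload magnitude and zeroes the others, then applies the spec to self.
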(event Ability|EventActivateAbility
  (bind _returnvalue (Ability|GetAbilitySystemComponentfromActorInfo))
  (bind _payload (Ability|Tasks|WaitGameplayEvent "(TagName=\"Attributes\")" 0 false false)
    (:EventReceived
      (Variables|Default|SetEventTag (.EventTag (Utilities|Struct|BreakGameplayEventData _payload)))
      (Variables|Default|SetEventMagnitude (.EventMagnitude (Utilities|Struct|BreakGameplayEventData _payload)))
      (Variables|Default|SetSpec (GameplayEffects|MakeOutgoingSpec _returnvalue (Variables|Default|GetEventBasedEffectClass) 1.0 (GameplayEffects|MakeEffectContext _returnvalue)))
      (for _array_element (Variables|Default|GetEventTags)
        (bind _output_get (Variables|Default|SetCurrentTag _array_element))
        (if (GameplayTags|MatchesTag _output_get (Variables|Default|GetEventTag) true)
          (Ability|GameplayEffect|AssignTagSetbyCallerMagnitude (Variables|Default|GetSpec) (Variables|Default|GetEventTag) (Variables|Default|GetEventMagnitude))
          (else
            (Ability|GameplayEffect|AssignTagSetbyCallerMagnitude (Variables|Default|GetSpec) (Variables|Default|GetCurrentTag) 0.0))))
      (GameplayEffects|ApplyGameplayEffectSpecToSelf (Ability|GetAbilitySystemComponentfromActorInfo) (Variables|Default|GetSpec)))))