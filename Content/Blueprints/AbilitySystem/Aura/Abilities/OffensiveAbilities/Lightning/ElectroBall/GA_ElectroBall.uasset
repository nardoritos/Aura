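; Lightning gameplay ability that casts an electro ball, which periodically damages nearby enemies for a lifetime scaled by ability level.
; After commit, it faces the cursor target, plays the cast montage and spawns BP_ElectroBall at the weapon socket on the montage event.
; The ball's range delegates maintain an enemy map and looping shock cues attached to the ball.
; A looping timer damages mapped enemies, then destroys the ball and ends the ability.
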(event Custom|ApplyDamageToPulledTargets
  (if (< (Variables|Default|GetDamageTicksCounter) (Class|AuraAbilitySystemLibrary|GetValueatLevel (Variables|Default|GetLifeTime) (Math|Conversions|ToFloat(Integer) (Ability|GetAbilityLevel))))
    (Variables|Default|SetDamageTicksCounter (+ (Variables|Default|GetDamageTicksCounter) (Variables|Default|GetDamageDeltaTime)))
    (CallFunction|ApplyDamagetoPrimaryTargets)
    (else
      (Utilities|Time|ClearandInvalidateTimerbyHandle (Variables|Default|GetDamageTimer))
      (Default|PrepareDestroy (Variables|Default|GetSpawnedElectroBall))
      (Ability|EndAbility))))

(event Ability|EventActivateAbility
  (bind _returnvalue (Ability|GetAvatarActorfromActorInfo))
  (CallFunction|EnforceImplementsCombatInterface)
  (Ability|CommitAbility)
  (bind _datahandle (|TargetDataUnderMouse)
    (:ValidData
      (Variables|Default|SetTargetLocation (.Location (Collision|BreakHitResult (Ability|TargetData|GetHitResultfromTargetData _datahandle))))
      (Variables|Default|SetMouseHitActor (.HitActor (Collision|BreakHitResult (Ability|TargetData|GetHitResultfromTargetData _datahandle))))
      (Class|CombatInterface|UpdateFacingTarget(Message) (Ability|GetAvatarActorfromActorInfo) (Variables|Default|GetTargetLocation))
      (|PlayMontageandWaitProxy "None" "/Game/Assets/Characters/Aura/Animations/Abilities/AM_Cast_FireBolt.AM_Cast_FireBolt" 1.0 "None" true 1.0 0.0 false
        (:then
          (Ability|Tasks|WaitGameplayEvent "(TagName=\"Event.Montage.FireBolt\")" 0
            (:EventReceived
              (bind _returnvalue_2 (Class|CombatInterface|GetWeapon(Message) _returnvalue))
              (bind _returnvalue_3 (Game|SpawnActorfromClass :Class "/Game/Blueprints/AbilitySystem/Aura/Abilities/OffensiveAbilities/Lightning/ElectroBall/BP_ElectroBall.BP_ElectroBall_C" :SpawnTransform (Math|Transform|MakeTransform (Transformation|GetSocketLocation _returnvalue_2 (Variables|Default|GetWeaponSocket)) (Transformation|GetActorRotation _returnvalue) "1.000000,1.000000,1.000000") :CollisionHandlingOverride "AlwaysSpawn" :TransformScaleMethod "MultiplyWithRoot" :bShouldCauseDamage false :Instigator 0))
              (bind _output_get (Variables|Default|SetSpawnedElectroBall _returnvalue_3))
              (EventDispatchers|AssignOnEnemyEnterRange _output_get (EventDispatchers|CreateEvent :!event AddGameplayCuetoActor))
              (EventDispatchers|AssignOnEnemyExitsRange (Variables|Default|GetSpawnedElectroBall) (EventDispatchers|CreateEvent :!event RemoveGameplayCuefromActor))
              (bind _returnvalue_4 (Utilities|Time|SetTimerbyEvent (EventDispatchers|CreateEvent :!event Custom|ApplyDamageToPulledTargets) (Variables|Default|GetDamageDeltaTime) true))
              (Variables|Default|SetDamageTimer _returnvalue_4)
              (CallFunction|ApplyDamagetoPrimaryTargets)
              (Class|AuraDamageGameplayAbility|RemoveDefaultBlockedAbilities))))))))

(event Ability|EventOnEndAbility
  (params (bWasCancelled :type Boolean)))

(fn EnforceImplementsCombatInterface
  (if (Utilities|DoesObjectImplementInterface (Ability|GetAvatarActorfromActorInfo) "/Script/Aura.CombatInterface")
    (return)
    (else
      (Ability|EndAbility))))

(fn ApplyDamagetoTarget
  (params (Enemy :type Combat%20Interface%20Interface)))

(fn AddGameplayCuetoActor
  (params (Enemy :type Actor%20Object%20Reference))
  (if (not (Utilities|Map|Contains (Variables|Default|GetPrimaryEnemies) Enemy)) ; Only add Cue if actor doesn't already have it
    (Development|PrintString "Added Additional Target")
    (bind _output_get (LocalVariables|SetTargetActor Enemy))
    (Utilities|Map|Add (Variables|Default|GetPrimaryEnemies) _output_get (Ability|GameplayCue|MakeGameplayCueParameters :Location (Transformation|GetActorLocation (LocalVariables|GetTargetActor)) :SourceObject (LocalVariables|GetTargetActor) :TargetAttachComponent (Variables|/Script/Engine.Actor|GetRootComponent (Variables|Default|GetSpawnedElectroBall))))
    (GameplayCue|AddGameplayCueOnActor(Looping) (LocalVariables|GetTargetActor) "(TagName=\"GameplayCue.ShockLoop\")" (Ability|GameplayCue|MakeGameplayCueParameters :Location (Transformation|GetActorLocation (LocalVariables|GetTargetActor)) :SourceObject (LocalVariables|GetTargetActor) :TargetAttachComponent (Variables|/Script/Engine.Actor|GetRootComponent (Variables|Default|GetSpawnedElectroBall))))))

(fn RemoveGameplayCuefromActor
  (params (Enemy :type Actor%20Object%20Reference))
  (bind _primaryenemies (Variables|Default|GetPrimaryEnemies))
  (bind (_value _returnvalue) (Utilities|Map|Find _primaryenemies Enemy))
  (if _returnvalue
    (GameplayCue|RemoveGameplayCueOnActor(Looping) Enemy "(TagName=\"GameplayCue.ShockLoop\")" _value)
    (Utilities|Map|Remove (Variables|Default|GetPrimaryEnemies) Enemy)))

(fn ApplyDamagetoPrimaryTargets
  (bind _keys (Utilities|Map|Keys (Variables|Default|GetPrimaryEnemies)))
  (for _array_element _keys
    (Class|AuraAbilitySystemLibrary|ApplyDamageEffect (Class|AuraDamageGameplayAbility|MakeDamageEffectParamsfromClassDefaults _array_element "0, 0, 0" false "0, 0, 0" false "0, 0, 0" false 0.0))))