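; Electro ball actor for the lightning offensive ability, which tracks enemies entering and leaving its radius.
; On the server, a timeline grows it from zero to its original scale, and PrepareDestroy reverses that timeline to shrink it before destroying it.
; Sphere overlaps with EnemyInterface actors fire enter and exit range dispatchers.
; The construction script sizes both the collision sphere and the ElectroRadius component from Radius.
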(event OnComponentBeginOverlap(EnemyCollisionSphere)
  (params (OverlappedComponent :type Primitive%20Component%20Object%20Reference) (OtherActor :type Actor%20Object%20Reference) (OtherComp :type Primitive%20Component%20Object%20Reference) (OtherBodyIndex :type Integer) (bFromSweep :type Boolean) (SweepResult :type Hit%20Result%20Structure%20%28by%20ref%29))
  (if (Utilities|DoesObjectImplementInterface OtherActor "/Script/Aura.EnemyInterface")
    (Default|CallOnEnemyEnterRange OtherActor)))

(event OnComponentEndOverlap(EnemyCollisionSphere)
  (params (OverlappedComponent :type Primitive%20Component%20Object%20Reference) (OtherActor :type Actor%20Object%20Reference) (OtherComp :type Primitive%20Component%20Object%20Reference) (OtherBodyIndex :type Integer))
  (if (Utilities|DoesObjectImplementInterface OtherActor "/Script/Aura.EnemyInterface")
    (Default|CallOnEnemyExitsRange OtherActor)))

(event Custom|PrepareDestroy
  (bind (_direction _scalealpha) (Timeline|Timeline Reverse)
    (:Update
      (Transformation|SetActorScale3D (Math|Vector|Lerp(Vector) "0, 0, 0" (Variables|Default|GetOriginalScale) _scalealpha)))
    (:Finished
      (switch Utilities|FlowControl|Switch|SwitchonETimelineDirection _direction
        (:Backward
          (Actor|DestroyActor))))))

(event EventBeginPlay
  (|CallParentFunction)
  (Networking|SwitchHasAuthority
    (:Authority
      (Variables|Default|SetOriginalScale (Transformation|GetActorScale3D))
      (bind (_direction _scalealpha) (Timeline|Timeline Play)
        (:Update
          (Transformation|SetActorScale3D (Math|Vector|Lerp(Vector) "0, 0, 0" (Variables|Default|GetOriginalScale) _scalealpha)))
        (:Finished
          (switch Utilities|FlowControl|Switch|SwitchonETimelineDirection _direction
            (:Backward
              (Actor|DestroyActor))))))))

(fn ConstructionScript
  (Components|Sphere|SetSphereRadius (Variables|Default|GetEnemyCollisionSphere) (Variables|Default|GetRadius) true)
  (Transformation|SetRelativeScale3D (Variables|Default|GetElectroRadius) (Math|Conversions|ToVector(Float) (/ (Variables|Default|GetRadius) 1.5e+02))))