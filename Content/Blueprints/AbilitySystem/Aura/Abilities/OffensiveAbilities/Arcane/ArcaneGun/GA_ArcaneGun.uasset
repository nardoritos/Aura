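; Arcane Gun is a channeled offensive gameplay ability that fires projectiles from the weapon socket toward the mouse cursor while input is held.
; The cast montage's event locks movement, sets the shock-loop state and starts a looping timer.
; Each tick commits mana cost, re-reads the cursor target, turns the character and spawns a projectile.
; Input release or failed cost ends it, restoring movement and committing cooldown only if casting began.
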(event Custom|ApplyDamageAndCost
  ;[0.15 0.15 0.15 0.5] Apply Damage to Targets and Consume Mana Cost looping on a period of DamageDeltaTime
  (bind _returnvalue (Ability|CommitAbilityCost true))
  (if _returnvalue
    (bind _datahandle (|TargetDataUnderMouse)
      (:ValidData
        (CallFunction|StoreMouseInfo _datahandle)
        (CallFunction|RotateCharacter)
        (Class|AuraProjectileSpell|SpawnProjectile (Variables|Default|GetMouseHitLocation) (GameplayTags|MakeLiteralGameplayTag "(TagName=\"CombatSocket.Weapon\")") false 0.0)))
    (else
      (CallFunction|ClearTimerandEndAbility))))

(event Custom|ClearTimerAndEndAbility
  (Utilities|Time|ClearandInvalidateTimerbyHandle (Variables|Default|GetDamageAndCostTimer))
  (CallFunction|PreparetoEndAbility)
  ;[0.15 0.15 0.15 0.5] Do not consume Cooldown if Skill wasn't fully cast
  (if (Variables|Default|GetHasBegunCasting)
    (Ability|CommitAbilityCooldown false))
  (CallFunction|ClearReferences)
  (Ability|EndAbility))

(event Ability|EventActivateAbility
  ;[1 0 0.3464 0.5] Store Mouse Data Variables
  (CallFunction|EnforceImplementsCombatInterface)
  (bind _datahandle (|TargetDataUnderMouse)
    (:ValidData
      (CallFunction|StoreMouseInfo _datahandle)
      (Utilities|FlowControl|Sequence
        (:then_0
          ;[0.15 0.15 0.15 0.5] Prepare for Ability Activation
          (Class|CombatInterface|UpdateFacingTarget(Message) (Ability|GetAvatarActorfromActorInfo) (Variables|Default|GetMouseHitLocation)))
        (:then_1
          (|PlayMontageandWaitProxy "None" "/Game/Assets/Characters/Aura/Animations/Abilities/AM_Cast_ArcaneGun.AM_Cast_ArcaneGun" 1.0 "None" false 1.0 0.0 false
            (:then
              (Ability|Tasks|WaitGameplayEvent "(TagName=\"Event.Montage.ArcaneGun\")" 0 true
                (:EventReceived
                  (Variables|Default|SetHasBegunCasting true)
                  (CallFunction|InShockLoop)
                  (bind _returnvalue (Utilities|Time|SetTimerbyEvent (delegate Custom|ApplyDamageAndCost) (Variables|Default|GetDamageDeltaTime) true))
                  (Variables|Default|SetDamageAndCostTimer _returnvalue))))))
        (:then_2
          ;[0.15 0.15 0.15 0.5] Wait until Ability Input is Released, then Clear and Consume Cooldown
          (Ability|Tasks|WaitInputRelease false
            (:OnRelease
              (CallFunction|ClearTimerandEndAbility))))))))

(fn EnforceImplementsCombatInterface
  (if (Utilities|DoesObjectImplementInterface (Ability|GetAvatarActorfromActorInfo) "/Script/Aura.CombatInterface")
    (return)
    (else
      (Ability|EndAbility))))

(fn InShockLoop
  (bind _returnvalue (Ability|GetAvatarActorfromActorInfo))
  (Class|CombatInterface|SetinShockLoop(Message) _returnvalue true)
  (Pawn|Components|CharacterMovement|DisableMovement (Variables|/Script/Engine.Character|GetCharacterMovement (.AsAura%20Character%20Base (Utilities|Casting|CastToAuraCharacterBase _returnvalue)))))

(fn ClearReferences
  (Variables|Default|SetMouseHitLocation "0, 0, 0")
  (Variables|Default|SetCurrentMouseHitActor 0)
  (Variables|Default|SetHasBegunCasting false)
  (Variables|Default|SetDamageAndCostTimer ""))

(fn PreparetoEndAbility
  (bind _returnvalue (Ability|GetAvatarActorfromActorInfo))
  (Class|CombatInterface|SetinShockLoop(Message) _returnvalue false)
  (Pawn|Components|CharacterMovement|SetMovementMode (Variables|/Script/Engine.Character|GetCharacterMovement (.AsAura%20Character%20Base (Utilities|Casting|CastToAuraCharacterBase _returnvalue))) "MOVE_Walking" 0))

(fn StoreMouseInfo
  (params (HitResult :type Gameplay%20Ability%20Target%20Data%20Handle%20Structure%20%28by%20ref%29))
  (bind _returnvalue (Ability|TargetData|GetHitResultfromTargetData HitResult))
  (bind (_bblockinghit _binitialoverlap _time _distance _location _impactpoint _normal _impactnormal _physmat _hitactor) (Collision|BreakHitResult _returnvalue))
  (Variables|Default|SetMouseHitLocation _impactpoint)
  (Variables|Default|SetCurrentMouseHitActor _hitactor))

(fn RotateCharacter
  (bind _returnvalue (Ability|GetAvatarActorfromActorInfo))
  (Default|Interpto (.AsBP%20Playable%20Character (Utilities|Casting|CastToBP_PlayableCharacter _returnvalue)) (Math|Rotator|FindLookatRotation (Transformation|GetActorLocation _returnvalue) (Variables|Default|GetMouseHitLocation))))