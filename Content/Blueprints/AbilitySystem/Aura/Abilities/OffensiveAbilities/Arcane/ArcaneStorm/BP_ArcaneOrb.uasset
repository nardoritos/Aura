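; BP_ArcaneOrb is an orb actor for the Arcane Storm offensive ability that plays a grow-in animation when it spawns.
; BeginPlay derives start and end points from the Sphere's relative transform, with the end a short distance along its forward vector.
; GrowTimeline lerps the actor's relative location between those points while driving its scale, then calls AnimationFinished when complete.
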(event EventBeginPlay
  (bind _sphere (Variables|Default|GetSphere))
  (bind _returnvalue (Transformation|GetRelativeTransform _sphere))
  (Variables|Default|SetOriginalLocation (.location _returnvalue))
  (Variables|Default|SetFinalLocation (+ (Variables|Default|GetOriginalLocation) (* (Math|Vector|GetForwardVector (.rotation _returnvalue)) 75.0)))
  (bind (_direction _location _scale) (Timeline|GrowTimeline PlayFromStart)
    (:Update
      (Utilities|FlowControl|Sequence
        (:then_0
          (Transformation|SetActorRelativeLocation (Math|Vector|Lerp(Vector) (Variables|Default|GetOriginalLocation) (Variables|Default|GetFinalLocation) _location)))
        (:then_1
          (Transformation|SetActorScale3D (Math|Conversions|ToVector(Float) _scale)))))
    (:Finished
      (Class|AuraStandbyProjectile|AnimationFinished))))

(fn ConstructionScript)