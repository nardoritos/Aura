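; Arcane Storm offensive ability that spawns projectiles on an orb holder at the caster and deals area damage where each hits.
; Activation commits cost, plays the cast montage, then waits for its gameplay event to spawn projectiles and bind hit callbacks.
; Each hit damages nearby live players except the caster, triggering shard cues and a burst effect.
; Cooldown is deferred until the last projectile hits, when the holder is destroyed and the ability ends.
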(event Custom|CheckRemainingProjectiles
  (if (== (Utilities|Array|Length (Variables|Default|GetSpawnedProjectiles)) 0)
    (Actor|DestroyActor (Variables|Default|GetOrbHolder))
    (Ability|CommitAbilityCooldown false)
    (Ability|EndAbility)))

(event Ability|EventActivateAbility
  (bind _returnvalue (Ability|GetAvatarActorfromActorInfo))
  (Ability|CommitAbilityCost false)
  (|PlayMontageandWaitProxy "None" "/Game/Assets/Characters/Aura/Animations/Abilities/AM_Cast_ArcaneStorm.AM_Cast_ArcaneStorm" 1.0 "None" true 1.0 0.0 false
    (:then
      (Ability|Tasks|WaitGameplayEvent "(TagName=\"Event.Montage.ArcaneStorm\")" 0
        (:EventReceived
          (bind _returnvalue_2 (Game|SpawnActorfromClass "/Game/Blueprints/AbilitySystem/Aura/Abilities/OffensiveAbilities/Arcane/ArcaneStorm/BP_OrbHolder.BP_OrbHolder_C" (Math|Transform|MakeTransform (Transformation|GetActorLocation _returnvalue) "0, 0, 0" "1.000000,1.000000,1.000000") "Undefined" "MultiplyWithRoot" 0 _returnvalue 0))
          (bind _output_get (Variables|Default|SetOrbHolder _returnvalue_2))
          (bind _returnvalue_3 (Class|AuraStandbyProjectileSpell|SpawnProjectiles _output_get))
          (bind _output_get_2 (Variables|Default|SetSpawnedProjectiles _returnvalue_3))
          (for _array_element _output_get_2
            (EventDispatchers|AssignOnProjectileHit _array_element (EventDispatchers|CreateEvent :!event OnProjectileHitEvent))))))))

(fn OnProjectileHitEvent
  (params (HittingProjectile :type Aura%20Standby%20Projectile%20Object%20Reference) (HitLocation :type Transform))
  (bind _location (Math|Transform|BreakTransform HitLocation))
  (Utilities|Array|RemoveItem (Variables|Default|GetSpawnedProjectiles) HittingProjectile)
  (bind _outoverlappingactors (Class|AuraAbilitySystemLibrary|GetLivePlayersWithinRadius self (Utilities|Array|MakeArray (Ability|GetAvatarActorfromActorInfo)) 225.0 _location false))
  (for _array_element _outoverlappingactors
    (bind _output_get (LocalVariables|SetCurrentEnemyHit _array_element))
    (bind _returnvalue (Class|AuraAbilitySystemLibrary|ApplyDamageEffect (Class|AuraDamageGameplayAbility|MakeDamageEffectParamsfromClassDefaults _output_get "0, 0, 0" true "0, 0, 0" false "0, 0, 0" false 0.0)))
    (GameplayCue|ExecuteGameplayCueOnActor(Burst) (LocalVariables|GetCurrentEnemyHit) "(TagName=\"GameplayCue.ArcaneShards\")" (Ability|GameplayCue|MakeGameplayCueParameters 0.0 0.0 _returnvalue)))
  (Niagara|SpawnSystematLocation "/Game/Assets/MegaMagicVFXBundle/VFX/MagicShieldsVFX/VFX/DefaultVersions/ArcaneShield/Systems/N_ArcaneShield_Burst.N_ArcaneShield_Burst" _location)
  (CallFunction|CheckRemainingProjectiles)
  (return))