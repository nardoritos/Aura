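; BP_FireNado is the actor for the FireNado fire ability, animating the tornado's appearance and removal by scale.
; On BeginPlay, only with authority, it stores its original scale and plays a timeline that grows it from zero to that scale.
; PrepareDestroy reverses the same timeline, shrinking the actor and destroying it once the backward play finishes.
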(event Custom|PrepareDestroy
  (bind (_direction _scalealpha) (Timeline|ScaleTimeline Reverse)
    (:Update
      (Transformation|SetActorScale3D (Math|Vector|Lerp(Vector) "0, 0, 0" (Variables|Default|GetOriginalScale) _scalealpha)))
    (:Finished
      (switch Utilities|FlowControl|Switch|SwitchonETimelineDirection _direction
        (:Backward
          (Actor|DestroyActor))))))

(event EventBeginPlay
  (|CallParentFunction)
  (Networking|SwitchHasAuthority
    (:Authority
      (Variables|Default|SetOriginalScale (Transformation|GetActorScale3D))
      (bind (_direction _scalealpha) (Timeline|ScaleTimeline Play)
        (:Update
          (Transformation|SetActorScale3D (Math|Vector|Lerp(Vector) "0, 0, 0" (Variables|Default|GetOriginalScale) _scalealpha)))
        (:Finished
          (switch Utilities|FlowControl|Switch|SwitchonETimelineDirection _direction
            (:Backward
              (Actor|DestroyActor))))))))

(fn ConstructionScript)