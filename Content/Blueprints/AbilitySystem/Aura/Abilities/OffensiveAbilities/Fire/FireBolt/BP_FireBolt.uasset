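; BP_FireBolt is the Fire Bolt ability's projectile actor.
; On BeginPlay it waits briefly before setting its collision sphere to query-only.
; Each tick compares its location with the previous frame's as a safety check for a stalled bolt, such as when its homing target becomes invalid.
; If movement falls to the minimum per-frame distance or below, it plays impact sound and explosion effects, then destroys itself.
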(event EventBeginPlay
  (Utilities|FlowControl|Delay 0.11)
  (Collision|SetCollisionEnabled (Variables|Default|GetSphere) "QueryOnly"))

(event EventTick
  (params (DeltaSeconds :type Float%20%28single-precision%29))
  ;[0.15 0.15 0.15 0.5] DestroyActor if Distance is less than MinDistancePerFrame / Homing Target is not valid anymore
  (CallFunction|SafeCheckDistanceBetweenFrames))

(fn ConstructionScript)

(fn SafeCheckDistanceBetweenFrames
  (Variables|Default|SetLastFrameLocation (Variables|Default|GetCurrentFrameLocation))
  (Variables|Default|SetCurrentFrameLocation (Transformation|GetActorLocation))
  (if (<= (Math|Vector|VectorLength (- (Variables|Default|GetCurrentFrameLocation) (Variables|Default|GetLastFrameLocation))) (Variables|Default|GetMinDistancePerFrame))
    (Audio|SpawnSoundatLocation "/Game/Assets/Sounds/Abilities/FireBolt/sfx_FireBolt_Impact.sfx_FireBolt_Impact" (Variables|Default|GetCurrentFrameLocation) "0, 0, 0" 1.0 1.0 0.0 0 0)
    (Niagara|SpawnSystematLocation "/Game/Assets/Effects/Projectiles/FireExplosion/NS_FireExplosion.NS_FireExplosion" (Variables|Default|GetCurrentFrameLocation))
    (Actor|DestroyActor)))