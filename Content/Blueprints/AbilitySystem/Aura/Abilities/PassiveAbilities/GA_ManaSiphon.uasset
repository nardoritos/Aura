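; Passive mana siphon ability that spawns a soul which homes to a killer to grant mana regen.
; On activation it waits for the ManaSiphon Soul gameplay event, then asks the instigator pawn for its killing actor.
; It spawns BP_ManaSiphon_Soul with level-based regen params targeting that actor.
; The random-point node feeding the spawn location is never executed.
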(event Ability|EventActivateAbility
  (bind _payload (Ability|Tasks|WaitGameplayEvent "(TagName=\"Abilities.Passive.ManaSiphon.Soul\")" 0)
    (:EventReceived
      (CallFunction|SpawnManaSiphonSoul _payload))))

(fn SpawnManaSiphonSoul
  (params (GameplayEventData :type Gameplay%20Event%20Data%20Structure%20%28by%20ref%29))
  (bind _aspawn (Utilities|Casting|CastToPawn (Utilities|Struct|BreakGameplayEventData GameplayEventData)))
  (bind _output_get (LocalVariables|SetInstigatorPawn _aspawn))
  (bind _returnvalue (Class|EnemyInterface|GetKillingActor(Message) _output_get))
  (LocalVariables|SetKillingActor _returnvalue)
  (bind _returnvalue_2 (Game|SpawnActorfromClass :Class "/Game/Blueprints/AbilitySystem/Aura/Abilities/PassiveAbilities/ManaSiphon/BP_ManaSiphon_Soul.BP_ManaSiphon_Soul_C" :SpawnTransform (Math|Transform|MakeTransform (stale _returnvalue) "0, 0, 0" "1.000000,1.000000,1.000000") :CollisionHandlingOverride "Undefined" :TransformScaleMethod "MultiplyWithRoot" :bShouldCauseDamage false :HealingEffectParams (Utilities|Struct|MakeRegenEffectParams (LocalVariables|GetKillingActor) "(TagName=\"Attributes.Meta.IncomingManaRegen\")" "/Game/Blueprints/AbilitySystem/Aura/Effects/GE_Regen.GE_Regen_C" (Ability|GetAbilitySystemComponent (LocalVariables|GetKillingActor)) (Variables|Default|GetRegenAmount) (Math|Conversions|ToFloat(Integer) (Ability|GetAbilityLevel))) :Instigator (LocalVariables|GetInstigatorPawn)))
  (Class|AuraProjectileBase|SetHomingTarget _returnvalue_2 (LocalVariables|GetKillingActor) (Transformation|GetActorLocation (LocalVariables|GetKillingActor))))