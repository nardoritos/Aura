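; Halo of Protection passive gameplay ability that keeps an indefinite GE_HaloOfProtection effect on its avatar while active.
; Activation builds effect params from the Resilience attribute tag, a base magnitude and the ability level, then applies them to the avatar's ability system component.
; A successful application stores the effect handle, which OnEndAbility uses to remove all stacks.
; Debug prints report activation and whether the effect applied.
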(event Ability|EventActivateAbility
  (Development|PrintString "Hello")
  (bind (_appliedsuccessfully _returnvalue) (Class|AuraAbilitySystemLibrary|ApplyIndefiniteEffect (Utilities|Struct|MakeIndefiniteEffectParams "/Game/Blueprints/AbilitySystem/Aura/Abilities/PassiveAbilities/HaloOfProtection/GE_HaloOfProtection.GE_HaloOfProtection_C" (Ability|GetAbilitySystemComponent (Ability|GetAvatarActorfromActorInfo)) "(TagName=\"Attributes.Primary.Resilience\")" (Variables|Default|GetResistenceMagnitude) (Math|Conversions|ToFloat(Integer) (Ability|GetAbilityLevel)))))
  (if _appliedsuccessfully
    (Development|PrintString "Applied")
    (Variables|Default|SetHaloOfProtectionHandle _returnvalue)
    (else
      (Development|PrintString "Failed to Apply"))))

(event Ability|EventOnEndAbility
  (params (bWasCancelled :type Boolean))
  (Ability|RemoveGameplayEffectFromOwnerWithHandle (Variables|Default|GetHaloOfProtectionHandle)))