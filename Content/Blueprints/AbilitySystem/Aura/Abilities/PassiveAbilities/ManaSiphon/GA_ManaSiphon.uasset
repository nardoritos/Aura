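; GA_ManaSiphon is a passive gameplay ability that, despite its name, uses the Life Siphon event tag and soul actor.
; On each soul event, it spawns a non-damaging BP_LifeSiphon_Soul at the event instigator's location.
; The soul carries GE_Regen parameters scaled by ability level and homes in on the instigator's killer, whose ability system receives the regen.
; Debug prints log each event and killer.
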(event Ability|EventActivateAbility
  (bind _payload (Ability|Tasks|WaitGameplayEvent "(TagName=\"Abilities.Passive.LifeSiphon.Soul\")" 0)
    (:EventReceived
      (Development|PrintString "Received")
      (bind _returnvalue (Class|EnemyInterface|GetKillingActor(Message) (.Instigator (Utilities|Struct|BreakGameplayEventData _payload))))
      (Development|PrintString (Utilities|GetDisplayName _returnvalue))
      (bind _returnvalue_2 (Game|SpawnActorfromClass :Class "/Game/Blueprints/AbilitySystem/Aura/Abilities/PassiveAbilities/LifeSiphon/BP_LifeSiphon_Soul.BP_LifeSiphon_Soul_C" :SpawnTransform (Math|Conversions|ToTransform(Vector) (Transformation|GetActorLocation (.Instigator (Utilities|Struct|BreakGameplayEventData _payload)))) :CollisionHandlingOverride "Undefined" :TransformScaleMethod "MultiplyWithRoot" :bShouldCauseDamage false :HealingEffectParams (Utilities|Struct|MakeRegenEffectParams _returnvalue "(TagName=\"\")" "/Game/Blueprints/AbilitySystem/Aura/Effects/GE_Regen.GE_Regen_C" (Ability|GetAbilitySystemComponent _returnvalue) (Math|Conversions|ToFloat(Integer) (+ (* (Ability|GetAbilityLevel) 10) 40))) :Instigator (.AsPawn (Utilities|Casting|CastToPawn (.Instigator (Utilities|Struct|BreakGameplayEventData _payload))))))
      (Class|AuraProjectileBase|SetHomingTarget _returnvalue_2 _returnvalue (Transformation|GetActorLocation _returnvalue)))))