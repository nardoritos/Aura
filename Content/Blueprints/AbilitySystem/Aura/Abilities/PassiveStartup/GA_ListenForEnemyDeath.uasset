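; Passive startup gameplay ability that listens for enemy death events and relays them to the Life Siphon and Mana Siphon passives.
; On activation it waits for the EnemyDeath gameplay event and passes the payload to OnEnemyKilled.
; That function scans the owned tags on the payload target's ASC, sending a matching Soul event with the same payload to the avatar.
; SendEventLifeSiphonSoul is an empty stub.
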(event Ability|EventActivateAbility
  (bind _payload (Ability|Tasks|WaitGameplayEvent "(TagName=\"Abilities.EnemyDeath\")" 0)
    (:EventReceived
      (CallFunction|OnEnemyKilled _payload))))

(fn SendEventLifeSiphonSoul
  (params (GameplayEventData :type Gameplay%20Event%20Data%20Structure%20%28by%20ref%29)))

(fn OnEnemyKilled
  (params (GameplayEventData :type Gameplay%20Event%20Data%20Structure%20%28by%20ref%29))
  (bind _target (Utilities|Struct|BreakGameplayEventData GameplayEventData))
  (bind _returnvalue (Ability|GetAbilitySystemComponent _target))
  (Utilities|IsValid _returnvalue
    (:Is%20Valid
      (for _array_element (GameplayTags|BreakGameplayTagContainer (GameplayTags|GetOwnedGameplayTags _returnvalue :!class /Script/GameplayTags.BlueprintGameplayTagLibrary))
        (|SwitchGameplayTag _array_element
          (:Abilities.Passive.LifeSiphon
            (Ability|SendGameplayEventtoActor (Ability|GetAvatarActorfromActorInfo) "(TagName=\"Abilities.Passive.LifeSiphon.Soul\")" GameplayEventData))
          (:Abilities.Passive.ManaSiphon
            (Ability|SendGameplayEventtoActor (Ability|GetAvatarActorfromActorInfo) "(TagName=\"Abilities.Passive.ManaSiphon.Soul\")" GameplayEventData)))))))