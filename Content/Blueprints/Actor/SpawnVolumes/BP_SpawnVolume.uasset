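; Spawn volume actor that references a set of spawn points and visualizes its links to them for debugging.
; The construction script destroys previous arrows, then, if ShowDebug is on, adds an arrow component for each valid spawn point.
; Each arrow starts at the volume, rotated toward its point with length scaled to the distance.
; BeginPlay only turns ShowDebug off; this file contains no spawning logic.
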(event EventBeginPlay
  (Variables|AuraEnemySpawnVolume|Debug|SetShowDebug false))

(event Collision|EventActorBeginOverlap
  (params (OtherActor :type Actor%20Object%20Reference)))

(event EventTick
  (params (DeltaSeconds :type Float%20%28single-precision%29)))

(fn ConstructionScript
  (CallFunction|DebugDrawtoSpawns))

(fn DebugDrawtoSpawns
  (bind _returnvalue (Transformation|GetActorLocation))
  (for _array_element (Variables|AuraEnemySpawnVolume|Debug|GetViewArrows)
    (Utilities|IsValid _array_element
      (:Is%20Valid
        (Components|DestroyComponent _array_element))))
  (Utilities|Array|Clear (Variables|AuraEnemySpawnVolume|Debug|GetViewArrows))
  (if (Variables|AuraEnemySpawnVolume|Debug|GetShowDebug)
    (for _array_element_2 (Variables|Default|GetSpawnPoints)
      (Utilities|IsValid _array_element_2
        (:Is%20Valid
          (bind _returnvalue_2 (AddComponent|AddArrowComponent true))
          (Utilities|Array|AddUnique (Variables|AuraEnemySpawnVolume|Debug|GetViewArrows) _returnvalue_2)
          (Variables|/Script/Engine.ArrowComponent|SetArrowLength _returnvalue_2 (/ (Math|Vector|Distance(Vector) _returnvalue (Transformation|GetActorLocation _array_element_2)) (Variables|/Script/Engine.ArrowComponent|GetArrowSize _returnvalue_2)))
          (Transformation|SetWorldLocationAndRotation _returnvalue_2 (Transformation|GetActorLocation) (Math|Rotator|FindLookatRotation _returnvalue (Transformation|GetActorLocation _array_element_2)) false false))))))