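; BP_LootItem is a loot actor that flies out to a destination, then idles there.
; SetDestinationandAnimate builds a runtime spline with a raised midpoint and a small end bounce, which PositionTimeline follows while scaling the item up from zero.
; On landing it enables collision and starts PlayIdleAnimation, a looping hover and spin whose randomized timeline play rate varies the bob between items.
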(event EventSetDestinationandAnimate
  (params (InDestination :type Vector :default "0, 0, 0"))
  (Variables|Default|SetDestination InDestination)
  (Variables|Default|SetOriginalLocation (Transformation|GetActorLocation))
  (CallFunction|SetSplinePoints)
  (bind (_direction _movealpha _scalealpha) (Timeline|PositionTimeline PlayFromStart)
    (:Update
      (Transformation|SetActorLocation (Spline|GetLocationatTime (Variables|Default|GetSpline) _movealpha "World" false) false false)
      (Transformation|SetActorScale3D (Math|Vector|Lerp(Vector) "0, 0, 0" "1.000000,1.000000,1.000000" _scalealpha)))
    (:Finished
      (Class|AuraEffectActor|SetCollisionState true)
      (Class|AuraEffectActor|PlayIdleAnimation))))

(event EventPlayIdleAnimation
  (bind _idletimeline (Variables|Default|GetIdleTimeline))
  (Variables|Default|SetOriginalLocation (Transformation|GetActorLocation))
  (Variables|Default|SetOriginalRotation (Transformation|GetActorRotation))
  (Utilities|IsValid _idletimeline
    (:Is%20Valid
      (Components|Timeline|SetPlayRate _idletimeline (Math|Random|RandomFloatinRange 0.8 1.1))
      (bind _ztranslation (Timeline|IdleTimeline PlayFromStart)
        (:Update
          (Utilities|IsValid self
            (:Is%20Valid
              (Transformation|SetActorLocation (Math|Vector|MakeVector (.x (Variables|Default|GetOriginalLocation)) (.y (Variables|Default|GetOriginalLocation)) (Math|Float|Lerp (.z (Variables|Default|GetOriginalLocation)) (+ (.z (Variables|Default|GetOriginalLocation)) 25.0) _ztranslation)) false false)
              (Transformation|AddActorLocalRotation "0.000000,0.500000,0.000000" false false))))
        (:Finished
          (Timeline|IdleTimeline PlayFromStart))))))

(fn ConstructionScript)

(fn SetSplinePoints
  (bind _originallocation (Variables|Default|GetOriginalLocation))
  (bind _returnvalue (AddComponent|AddSplineComponent true))
  (bind _output_get (Variables|Default|SetSpline _returnvalue))
  (Variables|/Script/Engine.SplineComponent|SetDuration _output_get 1.0)
  (Spline|SetSplinePoints _output_get (Utilities|Array|MakeArray _originallocation (+ (* (+ _originallocation (Variables|Default|GetDestination)) 0.5) "0.000000,0.000000,100.000000") (Variables|Default|GetDestination) (+ (Variables|Default|GetDestination) "0.000000,0.000000,25.000000") (Variables|Default|GetDestination)) "World" true))