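; BP_FlamePillar is a flame pillar actor whose fire light flickers continuously.
; On BeginPlay it randomly picks one of two flame intensity timelines and plays it from the start.
; Each timeline update scales the FireLight component's intensity from BaseIntensity.
; When a timeline finishes, it triggers another random pick, so the flicker loops with varying patterns.
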(event Custom|AnimateLight
  (params (Selection :type Integer))
  (switch int Selection
    (:Default
      (bind _flameintensity (Timeline|FlameIntensityTimeline1 PlayFromStart)
        (:Update
          (CallFunction|UpdateLightIntensity _flameintensity))
        (:Finished
          (CallFunction|ChooseLight))))
    (:0
      (Timeline|FlameIntensityTimeline1 PlayFromStart))
    (:1
      (bind _flameintensity_2 (Timeline|FlameIntensityTimeline2 PlayFromStart)
        (:Update
          (CallFunction|UpdateLightIntensity _flameintensity_2))
        (:Finished
          (CallFunction|ChooseLight))))))

(event Custom|ChooseLight
  (CallFunction|AnimateLight (Math|Random|RandomIntegerinRange 0 1)))

(event EventBeginPlay
  (CallFunction|ChooseLight))

(fn ConstructionScript)

(fn UpdateLightIntensity
  (params (IntensityMultiplier :type Float%20%28double-precision%29))
  (Rendering|Components|Light|SetIntensity (Variables|Default|GetFireLight) (* IntensityMultiplier (Variables|Default|GetBaseIntensity))))