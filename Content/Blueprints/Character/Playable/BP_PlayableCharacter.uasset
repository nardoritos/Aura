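; BP_PlayableCharacter is the playable character Blueprint, handling camera obstruction fading, a motion-warp facing target and an animation-loop flag.
; Its construction script sizes and offsets the FadeCameraCollision box from the camera boom's arm length.
; Overlaps with that box send fade-out and fade-in messages to actors implementing BI_FadeInterface.
; Custom events update the "FacingTarget" warp location and set InAnimationLoop for a shock loop.
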(event OnComponentBeginOverlap(FadeCameraCollision)
  (params (OverlappedComponent :type Primitive%20Component%20Object%20Reference) (OtherActor :type Actor%20Object%20Reference) (OtherComp :type Primitive%20Component%20Object%20Reference) (OtherBodyIndex :type Integer) (bFromSweep :type Boolean) (SweepResult :type Hit%20Result%20Structure%20%28by%20ref%29))
  (if (Utilities|DoesObjectImplementInterface OtherActor "/Game/Blueprints/Actor/FadeActor/BI_FadeInterface.BI_FadeInterface_C")
    (Class|BIFadeInterface|FadeOut(Message) OtherActor)))

(event OnComponentEndOverlap(FadeCameraCollision)
  (params (OverlappedComponent :type Primitive%20Component%20Object%20Reference) (OtherActor :type Actor%20Object%20Reference) (OtherComp :type Primitive%20Component%20Object%20Reference) (OtherBodyIndex :type Integer))
  (if (Utilities|DoesObjectImplementInterface OtherActor "/Game/Blueprints/Actor/FadeActor/BI_FadeInterface.BI_FadeInterface_C")
    (Class|BIFadeInterface|Fadein(Message) OtherActor)))

(event EventSetinShockLoop
  (params (bInLoop :type Boolean))
  (Variables|Default|SetInAnimationLoop bInLoop))

(event EventUpdateFacingTarget
  (params (Target :type Vector%20%28by%20ref%29 :default "0, 0, 0"))
  (Class|MotionWarpingComponent|AddorUpdateWarpTargetfromLocation (Variables|Default|GetMotionWarping) "FacingTarget" Target))

(fn ConstructionScript
  (CallFunction|SetupCameraCollisionDistance))

(fn SetupCameraCollisionDistance
  (bind _fadecameracollision (Variables|Default|GetFadeCameraCollision))
  (bind _cameraboom (Variables|Default|GetCameraBoom))
  (bind _targetarmlength (Variables|/Script/Engine.SpringArmComponent|GetTargetArmLength _cameraboom))
  (Components|Box|SetBoxExtent _fadecameracollision (Math|Vector|MakeVector (/ _targetarmlength 4.0) 4e+01 4e+01) true)
  (Transformation|SetRelativeLocation _fadecameracollision (Math|Vector|MakeVector (/ _targetarmlength 2.0) 0.0 0.0) false false))