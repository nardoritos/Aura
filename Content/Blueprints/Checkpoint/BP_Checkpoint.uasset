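; Checkpoint actor that supplies visual feedback for its reached and enabled states.
; Reaching it plays a Glow timeline into the supplied dynamic material's Glow parameter, while SmokeVFX is active whenever the checkpoint is disabled.
; With ShowDebug on, the construction script rebuilds arrow components stretched toward each enemy volume that must be cleared before enabling.
; BeginPlay switches debug off and clears those arrows before calling the parent.
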(event EventUpdateEnabledState
  (params (bEnabled :type Boolean))
  (Components|Activation|SetActive (Variables|Default|GetSmokeVFX) (not bEnabled) true))

(event EventBeginPlay
  (Variables|Checkpoint|Debug|SetShowDebug false)
  (CallFunction|DebugDrawtoSpawnVolumes)
  (|CallParentFunction))

(event EventCheckpointReached
  (params (DynamicMaterialInstance :type Material%20Instance%20Dynamic%20Object%20Reference))
  (bind _glow (Timeline|Glow PlayFromStart)
    (:Update
      (Rendering|Material|SetScalarParameterValue DynamicMaterialInstance "Glow" _glow :!class /Script/Engine.MaterialInstanceDynamic))))

(fn ConstructionScript
  (CallFunction|DebugDrawtoSpawnVolumes))

(fn DebugDrawtoSpawnVolumes
  (bind _returnvalue (Transformation|GetActorLocation))
  (for _array_element (Variables|Checkpoint|Debug|GetViewArrows)
    (Components|DestroyComponent _array_element))
  (Utilities|Array|Clear (Variables|Checkpoint|Debug|GetViewArrows))
  (if (Variables|Checkpoint|Debug|GetShowDebug)
    (for _array_element_2 (Variables|Default|GetEnemyVolumesToClearBeforeEnabling)
      (Utilities|IsValid _array_element_2
        (:Is%20Valid
          (bind _returnvalue_2 (AddComponent|AddArrowComponent true))
          (Utilities|Array|AddUnique (Variables|Checkpoint|Debug|GetViewArrows) _returnvalue_2)
          (Variables|/Script/Engine.ArrowComponent|SetArrowLength _returnvalue_2 (/ (Math|Vector|Distance(Vector) _returnvalue (Transformation|GetActorLocation _array_element_2)) (Variables|/Script/Engine.ArrowComponent|GetArrowSize _returnvalue_2)))
          (Transformation|SetWorldLocationAndRotation _returnvalue_2 (Transformation|GetActorLocation) (Math|Rotator|FindLookatRotation _returnvalue (Transformation|GetActorLocation _array_element_2)) false false))))))