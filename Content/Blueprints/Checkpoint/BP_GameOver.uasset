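; BP_GameOver is a highlightable checkpoint actor that shows a NextLevelWidget and a bottom light while highlighted.
; It extends the parent's highlight and unhighlight events to toggle both components' visibility and an IsHighlighted flag.
; While that flag is set, Tick rotates the widget each frame to face the player camera, billboard style.
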(event EventHighlightActor
  (|CallParentFunction)
  (Rendering|SetVisibility (Variables|Default|GetNextLevelWidget) true false)
  (Variables|Default|SetbIsHighlighted true))

(event EventUnHighlightActor
  (|CallParentFunction)
  (Rendering|SetVisibility (Variables|Default|GetNextLevelWidget) false false)
  (Variables|Default|SetbIsHighlighted false))

(event EventTick
  (params (DeltaSeconds :type Float%20%28single-precision%29))
  (if (Variables|Default|GetbIsHighlighted)
    (Transformation|SetWorldRotation (Variables|Default|GetNextLevelWidget) (Math|Rotator|FindLookatRotation (Transformation|GetWorldLocation (Variables|Default|GetNextLevelWidget)) (Camera|GetCameraLocation (Game|GetPlayerCameraManager 0))) false false)))

(fn ConstructionScript)